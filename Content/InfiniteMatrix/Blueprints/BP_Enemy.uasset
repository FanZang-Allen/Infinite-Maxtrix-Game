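; BP_Enemy is an enemy actor that reacts to contact with the player and projectiles.
; An overlap of SM_Enemy with BP_Player calls the player's ProcessHit and destroys the enemy.
; An overlap with BP_Projectile raises the player's score, calls ChangeSpeed on the player and destroys the enemy.
; A separate Trigger component silently destroys the enemy when BP_Player overlaps it, without registering a hit or score.
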(event OnComponentBeginOverlap(SM_Enemy)
  (params (OverlappedComponent :type Primitive%20Component%20Object%20Reference) (OtherActor :type Actor%20Object%20Reference) (OtherComp :type Primitive%20Component%20Object%20Reference) (OtherBodyIndex :type Integer) (bFromSweep :type Boolean) (SweepResult :type Hit%20Result%20Structure%20%28by%20ref%29))
  (bind _player (Variables|Default|GetPlayer))
  (Utilities|FlowControl|Sequence
    (:then_0
      (Utilities|Casting|CastToBP_Player OtherActor)
      (Default|ProcessHit (Variables|Default|GetPlayer))
      (Actor|DestroyActor))
    (:then_1
      (Utilities|Casting|CastToBP_Projectile OtherActor)
      (Default|ChangeScore _player (+ (Variables|/Game/InfiniteMatrix/Blueprints/BP_Player.BP_Player_C|GetScore _player) 5))
      (Default|ChangeSpeed _player)
      (Actor|DestroyActor))))

(event OnComponentBeginOverlap(Trigger)
  (params (OverlappedComponent :type Primitive%20Component%20Object%20Reference) (OtherActor :type Actor%20Object%20Reference) (OtherComp :type Primitive%20Component%20Object%20Reference) (OtherBodyIndex :type Integer) (bFromSweep :type Boolean) (SweepResult :type Hit%20Result%20Structure%20%28by%20ref%29))
  (Utilities|Casting|CastToBP_Player OtherActor)
  (Actor|DestroyActor))

(event EventBeginPlay)

(event Collision|EventActorBeginOverlap
  (params (OtherActor :type Actor%20Object%20Reference)))

(event EventTick
  (params (DeltaSeconds :type Float%20%28single-precision%29)))

(fn ConstructionScript)